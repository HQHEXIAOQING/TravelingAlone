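; BPS_Roll is a skill that rolls the instigating character forward, repeatable up to RollMaxNum times.
; Each roll line-traces along the forward vector and stops at the hit point or full Distance.
; A looping timer interpolates the actor there without sweep.
; The last roll applies cooldown and ends immediately; earlier rolls do so after a retriggerable delay, ending only if no roll is in progress.
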(event `self.SkillTriggerRepeatedlyEvent`
  (params (NewHQSkillLInfo :type "HQSkillInfo Structure"))
  (bind _instigator (`self.Instigator`))
  (bind _returnvalue (`Actor.K2_GetActorLocation` _instigator))
  (bind _result (`/Engine/EditorBlueprintResources/StandardMacros.IncrementInt` (`self.RollNum`))
    (:`  `
      (if (not (> _result (`self.RollMaxNum`)))
        (`KismetSystemLibrary.K2_ClearAndInvalidateTimerHandle` (`self.LocationOffsetTimer`))
        (set `self.IsSucceed` false :!label _label)
        (set `self.CurrentLocation` _returnvalue)
        (bind _outhit (`KismetSystemLibrary.LineTraceSingle` :`Start` _returnvalue :`End` (+ _returnvalue (* (`Actor.GetActorForwardVector` _instigator) (`self.Distance`))) :`TraceChannel` "TraceTypeQuery1" :`DrawDebugType` "ForDuration" :`DrawTime` 2.0))
        (bind (_bblockinghit _binitialoverlap _time _distance _location _impactpoint _normal _impactnormal _physmat _hitactor _hitcomponent _hitbonename _bonename _hititem _elementindex _faceindex _tracestart _traceend) (`GameplayStatics.BreakHitResult` _outhit))
        (set `self.EndLocation` (select `bool` _bblockinghit :`false` _traceend :`true` _location))
        (bind _returnvalue_2 (`KismetSystemLibrary.K2_SetTimerDelegate` (delegate `Event_LocationOffset`) 0.01 true))
        (set `self.LocationOffsetTimer` _returnvalue_2)))))

(event `self.SkillStartEvent`
  (params (NewHQSkillLInfo :type "HQSkillInfo Structure"))
  (bind _astacharacter_base (cast `TACharacterBase` (`.Instigator` (break `HQSkillInfo` NewHQSkillLInfo))))
  (set `self.Instigator` _astacharacter_base)
  (set `self.RollNum` 1)
  (goto _label))

(event `Event_LocationOffset`
  (set `self.CurrentLocation` (`KismetMathLibrary.VInterpTo` (`self.CurrentLocation`) (`self.EndLocation`) (`GameplayStatics.GetWorldDeltaSeconds`) 10.0))
  (`Actor.K2_SetActorLocation` (`self.Instigator`) (`self.CurrentLocation`) false false)
  (if (<= (`KismetMathLibrary.Vector_Distance` (`self.CurrentLocation`) (`self.EndLocation`)) 5.0)
    (`KismetSystemLibrary.K2_ClearAndInvalidateTimerHandle` (`self.LocationOffsetTimer`))
    (set `self.IsSucceed` true)
    (if (== (`self.RollNum`) (`self.RollMaxNum`))
      (`self.SkillApplyCoolDown` (`self.Max CD`))
      (`self.SkillEnd` true)
      (else
        (`KismetSystemLibrary.RetriggerableDelay` (`self.DurationTime`))
        (`self.SkillApplyCoolDown` (`self.Max CD`))
        (if (`self.IsSucceed`)
          (`self.SkillEnd` true))))))