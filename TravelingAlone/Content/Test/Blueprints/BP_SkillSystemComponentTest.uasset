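; Test Blueprint for the skill system component that shows a skill's remaining cooldown as on-screen debug text.
; The cooldown-apply event stores the latest skill ID, and the cooldown-end event clears it.
; Tick queries the residual cooldown for that single tracked ID and prints it whenever the lookup succeeds.
; BeginPlay and the skill activation event are empty.
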(event `self.ReceiveTick`
  (params (DeltaSeconds :type "Float (single-precision)"))
  (bind _cool_down_skill_id (`self.Cool Down Skill ID`))
  (bind (_bissucceed _returnvalue) (`self.GetResidueCoolDown` _cool_down_skill_id))
  (if _bissucceed
    (`KismetSystemLibrary.PrintString` (`KismetStringLibrary.Concat_StrStr` "技能：" (`KismetStringLibrary.Conv_NameToString` _cool_down_skill_id) "剩余CD：" (`KismetStringLibrary.Conv_DoubleToString` _returnvalue)))))

(event `self.ActivateSkillEvent`
  (params (CurrentActivateSkill :type "SkillProcessingObjectBase Object Reference")))

(event `self.SkillApplyCoolDownEvent`
  (params (CoolDownSkillID :type Name))
  (set `self.Cool Down Skill ID` CoolDownSkillID))

(event `self.SkillCoolDownEndEvent`
  (params (CoolDownSkillID :type Name))
  (set `self.Cool Down Skill ID` "None"))